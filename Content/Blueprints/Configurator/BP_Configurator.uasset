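; Product configurator actor that shows a selected product variant on a single mesh.
; On BeginPlay it registers with BP_TestGameMode, checks the Products data, shows the first variant and creates WBP_MainUI with mouse input.
; The widget's PartSelected event drives ActivateVariant, which swaps the static mesh and picks one of two metal frame materials for slot 0.
; ToggleUI plays the widget's open/close animation.
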(event `self.ReceiveBeginPlay`
  (bind _returnvalue (`GameplayStatics.GetPlayerController` 0))
  (`|ExecutionSequence`
    (:`then_0`
      ; Setting a reference for self in Game mode
      (bind _asbp_test_game_mode (cast `/Game/Blueprints/BP_TestGameMode` (`GameplayStatics.GetGameMode`))
        (:`then`
          (set `/Game/Blueprints/BP_TestGameMode.BP_Configurator` self _asbp_test_game_mode)
          (`self.Initialize`)
          ; Setup UI
          (`self.EnableInput` _returnvalue null)
          (bind _returnvalue_2 (`|CreateWidget` "/Game/UI/WBP_MainUI.WBP_MainUI_C"))
          (bind _output_get (set `self.UI` _returnvalue_2))
          (`UserWidget.AddToViewport` _output_get 0)
          (`WidgetBlueprintLibrary.SetInputMode_GameAndUIEx` _returnvalue _output_get "DoNotLock" false)
          (set `PlayerController.bShowMouseCursor` true _returnvalue))
        (:`CastFailed`
          (`KismetSystemLibrary.PrintString` "Warning: GameMode is Incorrect"))))
    (:`then_1`
      (bind _ui (`self.UI`)
        (:`then`
          (add `/Game/UI/WBP_MainUI.PartSelected` _ui (delegate `ToggleParts`)))
        (:`else`
          (`KismetSystemLibrary.PrintString` "Warning: UI not Initialized Properly"))))))

(event `ToggleParts`
  (params (ProductIndex :type Integer) (VariantIndex :type Integer) (MaterialIndex :type Integer))
  (`self.ActivateVariant` (`|GetArrayItem` (`self.Products`) ProductIndex) VariantIndex MaterialIndex))

(event `ToggleUI`
  (if (`self.bIsUI_Visible`)
    (bind _ui (`self.UI`)
      (:`then`
        (`/Game/UI/WBP_MainUI.PlayOpenCloseAnim` _ui "Reverse")
        (set `self.bIsUI_Visible` false))
      (:`else`))
    (else
      (bind _ui_2 (`self.UI`)
        (:`then`
          (`/Game/UI/WBP_MainUI.PlayOpenCloseAnim` _ui_2 "Forward")
          (set `self.bIsUI_Visible` true))
        (:`else`)))))

(fn `ActivateVariant`
  (params (Product :type "/Game/Blueprints/Configurator/Product Structure") (ProductIndex :type Integer) (MaterialIndex :type Integer))
  (bind _mesh (`self.Mesh`))
  (bind (_name _thumbnail _asset) (break `/Game/Blueprints/Configurator/ProductDetails` (`|GetArrayItem` (`.Variants_10_85004E4246551BC0B60DADBE46DAEBF7` (break `/Game/Blueprints/Configurator/Product` Product)) ProductIndex)))
  (`/Engine/EditorBlueprintResources/StandardMacros.IsValid` _asset
    (:`Is Valid`
      (`StaticMeshComponent.SetStaticMesh` _mesh _asset)
      (if (== MaterialIndex 0)
        (`PrimitiveComponent.SetMaterial` _mesh 0 "/Game/Configurator/Materials/Metal_frame.Metal_frame")
        (else
          (`PrimitiveComponent.SetMaterial` _mesh 0 "/Game/Configurator/Materials/Metal_frame1.Metal_frame1"))))
    (:`Is Not Valid`
      (`KismetSystemLibrary.PrintString` "Warning: Selected Variant Mesh is Not Valid!"))))

(fn `Initialize`
  (bind (_name _thumbnail _asset) (break `/Game/Blueprints/Configurator/ProductDetails` (`|GetArrayItem` (`.Variants_10_85004E4246551BC0B60DADBE46DAEBF7` (break `/Game/Blueprints/Configurator/Product` (`|GetArrayItem` (`self.Products`)))))))
  (if (== (`KismetArrayLibrary.Array_Length` (`self.Products`)) 0)
    (`KismetSystemLibrary.PrintString` "Warning: No Products Given")
    (else
      (for _array_element (`self.Products`)
        (for _array_element_2 (`.Variants_10_85004E4246551BC0B60DADBE46DAEBF7` (break `/Game/Blueprints/Configurator/Product` _array_element))
          (`/Engine/EditorBlueprintResources/StandardMacros.IsValid` (`.Asset_24_C0BEDF3148201426FCC904A0B15119D2` (break `/Game/Blueprints/Configurator/ProductDetails` _array_element_2))
            (:`Is Valid`
              (set `self.bSetupCorrect?` true))
            (:`Is Not Valid`
              (set `self.bSetupCorrect?` false)))))
      (if (`self.bSetupCorrect?`)
        (`/Engine/EditorBlueprintResources/StandardMacros.IsValid` _asset
          (:`Is Valid`
            (`StaticMeshComponent.SetStaticMesh` (`self.Mesh`) _asset))
          (:`Is Not Valid`
            (`KismetSystemLibrary.PrintString` "Warning: Configuration is not Correct.")))
        (else
          (`KismetSystemLibrary.PrintString` "Warning: Configuration is not Correct."))))))

(fn `UserConstructionScript`)
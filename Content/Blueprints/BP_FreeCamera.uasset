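; BP_FreeCamera is a free-flying camera pawn driven by Enhanced Input.
; On BeginPlay it adds the default mapping context, caches BP_TestGameMode and turns the camera toward the world origin.
; Look input drives controller yaw and pitch, while fly input moves the pawn along the camera's axes through FloatingPawnMovement.
; A toggle action shows or hides the game mode's configurator UI, and Escape quits the game.
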(event `self.ReceiveBeginPlay`
  ; Adding Mapping Context to scene
  (bind _asplayer_controller (cast `PlayerController` (`self.GetController`))
    (:`then`
      (`EnhancedInputSubsystemInterface.AddMappingContext` (pcsubsystem `EnhancedInputLocalPlayerSubsystem` _asplayer_controller) "/Game/Blueprints/Inputs/IMC_Default.IMC_Default" 0 (struct))
      (bind _asbp_test_game_mode (cast `/Game/Blueprints/BP_TestGameMode` (`GameplayStatics.GetGameMode`))
        (:`then`
          (set `self.GameMode` _asbp_test_game_mode)
          (`SceneComponent.K2_SetWorldRotation` (`self.Camera`) (`KismetMathLibrary.FindLookAtRotation` (`SceneComponent.K2_GetComponentLocation` (`self.SphereComponent`)) (`KismetMathLibrary.MakeVector` 0.0)) false false))
        (:`CastFailed`
          (`KismetSystemLibrary.PrintString` "Warning: Incorrect Game Selected"))))
    (:`CastFailed`
      (`KismetSystemLibrary.PrintString` "Warning: Can't create Input Mapping Context"))))

(event `EnhancedInput|/Game/Blueprints/Inputs/IA_Look`
  (params (ActionValue :type "Vector2D Structure") (ElapsedSeconds :type "Float (double-precision)") (TriggeredSeconds :type "Float (double-precision)") (InputAction :type "InputAction Object Reference" :default "/Game/Blueprints/Inputs/IA_Look.IA_Look"))
  ; Setup Look Controls
  (:`Triggered`
    (`self.AddControllerYawInput` ActionValue_X)
    (`self.AddControllerPitchInput` ActionValue_Y)))

(event `EnhancedInput|/Game/Blueprints/Inputs/IA_Fly`
  (params (ActionValue :type "Vector Structure") (ElapsedSeconds :type "Float (double-precision)") (TriggeredSeconds :type "Float (double-precision)") (InputAction :type "InputAction Object Reference" :default "/Game/Blueprints/Inputs/IA_Fly.IA_Fly"))
  (bind _camera (`self.Camera`))
  ; Setup Move Controls
  (:`Triggered`
    (`PawnMovementComponent.AddInputVector` (`self.FloatingPawnMovement`) (* (`SceneComponent.GetForwardVector` _camera) ActionValue_Y) false)
    (`PawnMovementComponent.AddInputVector` (`self.FloatingPawnMovement`) (* (`SceneComponent.GetRightVector` _camera) ActionValue_X) false)
    (`PawnMovementComponent.AddInputVector` (`self.FloatingPawnMovement`) (* (`SceneComponent.GetUpVector` _camera) ActionValue_Z) false)))

(event `EnhancedInput|/Game/Blueprints/Inputs/IA_ToggleUI`
  (params (ActionValue :type Boolean) (ElapsedSeconds :type "Float (double-precision)") (TriggeredSeconds :type "Float (double-precision)") (InputAction :type "InputAction Object Reference" :default "/Game/Blueprints/Inputs/IA_ToggleUI.IA_ToggleUI"))
  ; Setup UI Toggle
  (:`Started`
    (bind _gamemode (`self.GameMode`)
      (:`then`
        (bind _bp_configurator (`/Game/Blueprints/BP_TestGameMode.BP_Configurator` _gamemode)
          (:`then`
            (`/Game/Blueprints/Configurator/BP_Configurator.ToggleUI` _bp_configurator))
          (:`else`)))
      (:`else`))))

(event `Key|Escape`
  (params (Key :type "Key Structure"))
  (:`Released`
    (`KismetSystemLibrary.QuitGame` null "Quit")))

(fn `UserConstructionScript`)
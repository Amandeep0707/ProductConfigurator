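; BP_ProductLoader is a Blueprint meant to load a product mesh from configuration data, but its loading logic is currently unwired.
; BeginPlay and the Construction Script are empty, so nothing runs.
; The disconnected chain looks up the hardcoded "Bosco" row in ConfigurationData and async-loads its first configuration's first asset.
; It then sets the result on StaticMeshComponent, or prints a message if the row is missing.
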(event `self.ReceiveBeginPlay`)

(fn `UserConstructionScript`)